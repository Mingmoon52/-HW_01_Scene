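; Weapon Blueprint that handles automatic firing and magazine reloading.
; While the 開槍攻擊 input is held and ammo remains, a Delay-paced loop spawns a bullet at the weapon mesh's 子彈插槽 socket and decrements the magazine.
; Releasing the input clears the firing flag, ending the loop.
; The custom event 換彈匣 refills the magazine from reserve ammo, capped at what remains, and deducts that amount from the reserve.
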(event `InputAction|開槍攻擊`
  (params (Key :type "Key Structure"))
  ;[1 1 1] 開槍功能
  (:`Pressed`
    (set `self.開槍中` true)
    (if (and (> (`self.目前子彈數量`) 0) (`self.開槍中`)) :!label _label
      (`|SpawnActorFromClass` "/Game/BP/BP_子彈.BP_子彈_C" (`SceneComponent.GetSocketTransform` (`self.武器模型`) "子彈插槽" "RTS_World") "Undefined" "OverrideRootScale" null null) ; 生成子彈藍圖
      (set `self.目前子彈數量` (- (`self.目前子彈數量`) 1)) ; 開槍後子彈 -1
      (`KismetSystemLibrary.Delay` (`self.開槍間隔`))
      (goto _label)))
  (:`Released`
    (set `self.開槍中` false)))

(event `換彈匣`
  ;[0.7182 1 0.4166] 計算要補充幾顆子彈
  (set `self.要補充的子彈數量` (- (`self.彈匣尺寸`) (`self.目前子彈數量`))) ; 計算要補充的子彈數量 \n例 : 目前 10 彈匣 30 所以要補充 20
  ;[0.7182 1 0.4166] 判斷總數是否>=要補充的數量
  (if (not (>= (`self.子彈總數`) (`self.要補充的子彈數量`)))
    ;[0.7182 1 0.4166] 總數<要補充的數量 : 把剩餘總數補充
    (set `self.要補充的子彈數量` (`self.子彈總數`)))
  ;[0.7182 1 0.4166] 目前子彈以及總數更新
  (set `self.目前子彈數量` (+ (`self.目前子彈數量`) (`self.要補充的子彈數量`))) ; 補充子彈數練 ， \n例 : 目前 10 要補充為 20 補充後 目前為 30
  (set `self.子彈總數` (- (`self.子彈總數`) (`self.要補充的子彈數量`))) ; 扣除子彈總數 ， \n例  : 總數20 要補充為 20 補充後 總數為 0
)

(fn `UserConstructionScript`)