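; Game mode Blueprint that runs a minutes-and-seconds countdown timer.
; Tick feeds a one-second Delay, which ignores calls while pending, so the seconds variable (秒) drops about once per second.
; When seconds go below zero they wrap to 59 and minutes (分) decrease if above zero.
; Nothing stops the countdown at zero, so seconds keep cycling after minutes run out.
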(event `self.ReceiveTick`
  (params (DeltaSeconds :type "Float (single-precision)"))
  (`KismetSystemLibrary.Delay` 1.0) ; 延遲 : 等待所有設定的時間再執行後面的節點
  (bind _output_get (set `self.秒` (- (`self.秒`) 1)))
  (if (< _output_get 0)
    (set `self.秒` 59)
    (if (> (`self.分`) 0)
      (set `self.分` (- (`self.分`) 1)))))

(fn `UserConstructionScript`)