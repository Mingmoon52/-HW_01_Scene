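; Monster enemy that wanders at random until it sees the player, then chases them, and is destroyed when its health runs out.
; A looping AIMoveTo alternates between chasing the stored player and walking to random reachable points with random pauses.
; The pawn sensing component sets the chase flag and zeroes the pause, while a failed chase move restores wandering.
; Bullet overlaps on the capsule apply weapon damage and also set the chase flag.
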(event `self.感測元件.OnSeePawn`
  (params (Pawn :type "Pawn Object Reference"))
  ;[0.226 1 0.6262] 看到玩家後保存玩家資訊
  (bind `_asbp_玩家控制` (cast `/Game/BP/BP_玩家控制` Pawn))
  (set `self.玩家控制` `_asbp_玩家控制`)
  (set `self.是否看到玩家` true :!label _label)
  (set `self.停留時間最大值` 0.0) ; 看到玩家後馬上往玩家前進
  (`/Engine/EditorBlueprintResources/StandardMacros.DoOnce` false
    (:`Completed`
      ;[0.226 1 0.6262] 判斷有沒有看到玩家
      (if (`self.是否看到玩家`) :!label _label_2
        ;[0.226 1 0.6262] 看到玩家後 :追蹤玩家
        (`|AIMoveTo` self (0.0 0.0 0.0) (`self.玩家控制`) (`self.停止半徑`)
          (:`OnSuccess`
            (goto _label_2))
          (:`OnFail`
            (set `self.是否看到玩家` false)
            (set `self.停留時間最大值` 3.0) ; 恢復停留最大值為3
            (goto _label_2)))
        (else
          ;[0.226 1 0.6262] 沒有看到玩家：隨機走動
          (`|AIMoveTo` self (`NavigationSystemV1.K2_GetRandomReachablePointInRadius` (`SceneComponent.K2_GetComponentLocation` (`self.CapsuleComponent`)) (`self.隨機走動的半徑`) null null) null (`self.停止半徑`) ; AI 移動節點 : 移動到指定座標
            (:`then`
              ;[0.226 1 0.6262] 隨機停留
              (`KismetSystemLibrary.Delay` (* (`KismetMathLibrary.RandomFloat`) (`self.停留時間最大值`)))
              (goto _label_2))))))))

(event `self.ReceiveBeginPlay`
  (goto _label_2))

(event `self.CapsuleComponent.OnComponentBeginOverlap`
  (params (OverlappedComponent :type "PrimitiveComponent Object Reference") (OtherActor :type "Actor Object Reference") (OtherComp :type "PrimitiveComponent Object Reference") (OtherBodyIndex :type Integer) (bFromSweep :type Boolean) (SweepResult :type "HitResult Structure (by ref)"))
  ;[0.7809 0.3217 1] 受傷
  (bind `_asbp_子彈` (cast `/Game/BP/BP_子彈` OtherActor))
  (`self.受傷` (`/Game/BP/BP_子彈.目前武器傷害` `_asbp_子彈`))
  (goto _label))

(fn `UserConstructionScript`)

(fn `受傷`
  (params (`接收到的傷害值` :type "Float (double-precision)"))
  (bind _output_get (set `self.血量` (- (`self.血量`) `接收到的傷害值`)))
  (if (<= _output_get 0.0)
    (`self.K2_DestroyActor`)))